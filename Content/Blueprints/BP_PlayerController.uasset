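; Player controller Blueprint that handles the end of a game through Win and Lose events.
; Both events call ResetPlayer, which disables the character's input and zeroes its capsule's linear and angular physics velocity, then fade the camera out.
; After the fade, Win opens the WinScreen level, while Lose destroys the character and opens LoseScreen.
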(event `Win`
  ;[1 1 1] Win Event
  (`self.Reset Player`)
  (`PlayerCameraManager.StartCameraFade` :`self` (`GameplayStatics.GetPlayerCameraManager` 0) :`ToAlpha` 1.0 :`Duration` 3.0 :`bHoldWhenFinished` true)
  (`KismetSystemLibrary.Delay` 3.0)
  (`GameplayStatics.OpenLevel` "WinScreen"))

(event `Lose`
  ;[1 1 1] Lose Event
  (`self.Reset Player`)
  (`PlayerCameraManager.StartCameraFade` :`self` (`GameplayStatics.GetPlayerCameraManager` 0) :`ToAlpha` 1.0 :`Duration` 3.0 :`bHoldWhenFinished` true)
  (`KismetSystemLibrary.Delay` 3.0)
  (`self.K2_DestroyActor` (`GameplayStatics.GetPlayerCharacter` 0))
  (`GameplayStatics.OpenLevel` "LoseScreen"))

(fn `Reset Player`
  (bind _returnvalue (`GameplayStatics.GetPlayerCharacter` 0))
  (`self.DisableInput` _returnvalue null)
  (bind _asbp_player_character (cast `/Game/Blueprints/BP_PlayerCharacter` _returnvalue))
  (bind _capsulecomponent (`Character.CapsuleComponent` _asbp_player_character))
  (`PrimitiveComponent.SetPhysicsLinearVelocity` _capsulecomponent (0.0 0.0 0.0) false "None")
  (`PrimitiveComponent.SetPhysicsAngularVelocityInDegrees` _capsulecomponent (0.0 0.0 0.0) false "None"))

(fn `UserConstructionScript`)