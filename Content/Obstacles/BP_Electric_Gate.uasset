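; BP_Electric_Gate is an electrified obstacle that damages the player until enough items are collected to open it.
; It plays its gate audio on BeginPlay and applies damage when BP_PlayerCharacter begins overlapping its Box.
; CollectItem counts toward RequiredItems and, once reached, fires OpenGate a single time through a DoOnce.
; OpenGate destroys the gate FX and Box components, removing the visual and the hazard while leaving the audio untouched.
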(event `self.ReceiveBeginPlay`
  (`AudioComponent.Play` (`self.ElectricGate_Audio`) 0.0))

(event `Collect Item`
  ;[1 1 1] Collect Items
  (`/Engine/EditorBlueprintResources/StandardMacros.IncrementInt` (`self.currentItems`)
    (:`  `
      (if (>= (`self.currentItems`) (`self.requiredItems`))
        (`/Engine/EditorBlueprintResources/StandardMacros.DoOnce` false
          (:`Completed`
            (`self.Open Gate`)))))))

(event `Open Gate`
  ;[1 1 1] Open
  (`ActorComponent.K2_DestroyComponent` (`self.GateFX`))
  (`ActorComponent.K2_DestroyComponent` (`self.Box`)))

(event `self.Box.OnComponentBeginOverlap`
  (params (OverlappedComponent :type "PrimitiveComponent Object Reference") (OtherActor :type "Actor Object Reference") (OtherComp :type "PrimitiveComponent Object Reference") (OtherBodyIndex :type Integer) (bFromSweep :type Boolean) (SweepResult :type "HitResult Structure (by ref)"))
  ;[1 1 1] Damage Player
  (bind _asbp_player_character (cast `/Game/Blueprints/BP_PlayerCharacter` OtherActor))
  (`GameplayStatics.ApplyDamage` _asbp_player_character 50.0))

(fn `UserConstructionScript`)